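; Controller that finds the BlobPawn at BeginPlay, views through its camera and moves it each frame.
; Tick teleports the controller to an offset from the pawn, then moves the pawn by swept SetActorLocation, using only MaxWalkSpeed from CharacterMovement.
; GetMoveXY sums polled ZQSD (AZERTY) keys along the pawn's forward and right vectors with a gamepad term, whose axis math is left unwired.
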(event `self.ReceiveBeginPlay`
  (bind _returnvalue (`GameplayStatics.GetActorOfClass` "/Game/Blueprints/Actors/BlobPawn.BlobPawn_C"))
  (bind _output_get (set `self.ControlledPawn` _returnvalue))
  (`self.SetViewTargetWithBlend` (`ActorComponent.GetOwner` (`/Game/Blueprints/Actors/BlobPawn.Camera` _output_get))))

(event `self.ReceiveTick`
  (params (DeltaSeconds :type "Float (single-precision)"))
  (`self.K2_SetActorLocation` self (+ (`self.K2_GetActorLocation` (`self.ControlledPawn`)) (0.0 -50.0 50.0)) false true)
  (bind _movexy (`self.GetMoveXY` DeltaSeconds (`CharacterMovementComponent.MaxWalkSpeed` (`Character.CharacterMovement` (`self.ControlledPawn`))))
    (:`Exit`
      (`self.K2_SetActorLocation` (`self.ControlledPawn`) (+ _movexy (`self.K2_GetActorLocation` (`self.ControlledPawn`))) true false))))

(fn `UserConstructionScript`)