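; Falling platform actor that drops shortly after an actor with a BlobComponent hits it, then returns to its starting position.
; A hit starts a Tick-driven countdown whose thresholds select a brief delay, a fast descent, then a slower climb.
; Movement uses swept local offsets per frame, so speed depends on frame rate.
; Upon regaining its original height, it teleports to the saved location and re-arms.
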(event `self.ReceiveBeginPlay`
  (set `self.RemainingTime` 7.0)
  (set `self.OriginalPosition` (`self.K2_GetActorLocation`))
  (set `self.IsWaiting` true))

(event `self.ReceiveHit`
  (params (MyComp :type "PrimitiveComponent Object Reference") (Other :type "Actor Object Reference") (OtherComp :type "PrimitiveComponent Object Reference") (bSelfMoved :type Boolean) (HitLocation :type "Vector Structure") (HitNormal :type "Vector Structure") (NormalImpulse :type "Vector Structure") (Hit :type "HitResult Structure (by ref)"))
  (if (`KismetSystemLibrary.IsValid` (`self.GetComponentByClass` Other "/Game/Blueprints/Components/BlobComponent.BlobComponent_C"))
    (set `self.IsWaiting` false)))

(event `self.ReceiveTick`
  (params (DeltaSeconds :type "Float (single-precision)"))
  (if (not (`self.IsWaiting`))
    (bind _output_get (set `self.RemainingTime` (- (`self.RemainingTime`) DeltaSeconds)))
    (if (> _output_get 6.0)
      _
      (elif (> _output_get 4.7)
        (`self.K2_AddActorLocalOffset` (* (`KismetMathLibrary.Vector_Down`) (16.0 16.0 16.0)) true)
        (elif (< (`.Z` (`KismetMathLibrary.BreakVector3f` (`self.K2_GetActorLocation`))) (`.Z` (`KismetMathLibrary.BreakVector3f` (`self.OriginalPosition`))))
          (`self.K2_AddActorLocalOffset` (* (`KismetMathLibrary.Vector_Up`) (5.0 5.0 5.0)) true)
          (else
            (set `self.IsWaiting` true)
            (`self.K2_SetActorLocation` (`self.OriginalPosition`) false true)
            (set `self.RemainingTime` 7.0)))))))

(fn `UserConstructionScript`)