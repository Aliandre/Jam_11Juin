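; RoundMovingPlateform is a moving platform actor that shuttles back and forth along TargetOffset.
; Tick counts RemainingTime down from Period, then flips IsReversing and restarts the timer.
; While time remains, it teleports by plus or minus TargetOffset each frame without sweeping, with the sign picked by IsReversing.
; The step is not scaled by DeltaSeconds, so speed and travel distance depend on frame rate.
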(event `self.ReceiveBeginPlay`
  (set `self.RemainingTime` (`self.Period`)))

(event `self.ReceiveTick`
  (params (DeltaSeconds :type "Float (single-precision)"))
  (bind _output_get (set `self.RemainingTime` (- (`self.RemainingTime`) DeltaSeconds)))
  (if (> _output_get 0.0)
    (`self.K2_SetActorLocation` (+ (* (`self.TargetOffset`) (`KismetMathLibrary.SelectVector` (1.0 1.0 1.0) (-1.0 -1.0 -1.0) (`self.IsReversing`))) (`self.K2_GetActorLocation`)) false true)
    (else
      (set `self.IsReversing` (not (`self.IsReversing`)))
      (set `self.RemainingTime` (`self.Period`)))))

(fn `UserConstructionScript`)